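; BallPawn is a player-controlled rolling ball that can jump and keep a score.
; Move axes apply torque to BallMesh around control-rotation vectors, so it rolls relative to the view, while mouse and rate-scaled key inputs turn the controller.
; Jump adds an upward velocity impulse with a sound, then locks until any Hit event re-enables it, playing an impact sound.
; Escape quits the game, and IncrementScore adds to Score.
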(event `self.ReceiveBeginPlay`)

(event `self.ReceiveTick`
  (params (DeltaSeconds :type "Float (single-precision)")))

(event `Key|Escape`
  (params (Key :type "Key Structure"))
  ;[1 1 1] Quit the game
  (:`Pressed`
    (`KismetSystemLibrary.QuitGame` null "Quit")))

(event `InputAxis|Move_Forward`
  (params (AxisValue :type "Float (single-precision)"))
  ;[1 1 1] Move forwards and backwards
  (`PrimitiveComponent.AddTorqueInDegrees` (`self.Ball Mesh`) (* (* (`KismetMathLibrary.GetRightVector` (`self.GetControlRotation`)) (`self.Torque`)) AxisValue) "None" true))

(event `InputAxis|Look_Up_Rate`
  (params (AxisValue :type "Float (single-precision)"))
  ;[1 1 1] Up down arrow key input
  (`self.AddControllerPitchInput` (* AxisValue (`self.Turn_Rate`) (`GameplayStatics.GetWorldDeltaSeconds`))))

(event `InputAxis|Move_Right`
  (params (AxisValue :type "Float (single-precision)"))
  ;[1 1 1] Move left and right
  (`PrimitiveComponent.AddTorqueInDegrees` (`self.Ball Mesh`) (* (* (`KismetMathLibrary.GetForwardVector` (`KismetMathLibrary.MakeRotator` 0.0 0.0 (.yaw (`self.GetControlRotation`)))) (`self.Torque`)) AxisValue) "None" true))

(event `InputAxis|Turn_Rate`
  (params (AxisValue :type "Float (single-precision)"))
  ;[1 1 1] Left right arrow key input
  (`self.AddControllerYawInput` (* AxisValue (`self.Turn_Rate`) (`GameplayStatics.GetWorldDeltaSeconds`))))

(event `InputAction|Jump`
  (params (Key :type "Key Structure"))
  ;[1 1 1] Jumping
  (:`Pressed`
    (if (`self.CanJump`)
      (`PrimitiveComponent.AddImpulse` (`self.Ball Mesh`) (`KismetMathLibrary.MakeVector` 0.0 0.0 (`self.JumpPower`)) "None" true)
      (set `self.CanJump` false)
      (`GameplayStatics.PlaySound2D` "/Game/Retro_8Bit_Sounds/Jumping/Wavs/retro_jump_bounce_12.retro_jump_bounce_12" 1.0 1.0 0.0 null null))))

(event `self.ReceiveHit`
  (params (MyComp :type "PrimitiveComponent Object Reference") (Other :type "Actor Object Reference") (OtherComp :type "PrimitiveComponent Object Reference") (bSelfMoved :type Boolean) (HitLocation :type "Vector Structure") (HitNormal :type "Vector Structure") (NormalImpulse :type "Vector Structure") (Hit :type "HitResult Structure (by ref)"))
  ;[1 1 1] Can Jump setter
  (if (not (`self.CanJump`))
    (`GameplayStatics.PlaySound2D` "/Game/Retro_8Bit_Sounds/Impacts/Wavs/retro_impact_hit_11.retro_impact_hit_11" 1.0 1.0 0.0 null null))
  (set `self.CanJump` true))

(event `InputAxis|Look_Up`
  (params (AxisValue :type "Float (single-precision)"))
  ;[1 1 1] Mouse Camera Control
  (`self.AddControllerPitchInput` (* AxisValue -1.0)))

(event `InputAxis|Turn`
  (params (AxisValue :type "Float (single-precision)"))
  ;[1 1 1] Mouse Camera Control
  (`self.AddControllerYawInput` AxisValue))

(fn `IncrementScore`
  (params (InScore :type Integer))
  (set `self.Score` (+ InScore (`self.Score`))))

(fn `UserConstructionScript`)