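; Explosives pickup that penalizes the player, a child of a parent pickup class that it configures with negative points plus explosion sound and particle.
; On BeginPlay it sets those values and plays a sparking fuse sound at its location before calling the parent.
; When picked up by a BallPawn, it launches the ball with a radial velocity impulse centered slightly below itself, then runs the parent pickup logic.
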(event `self.ReceiveBeginPlay`
  (set `self.Points` -5)
  (set `self.OnPickupSound` "/Game/StarterContent/Audio/Explosion01.Explosion01")
  (set `self.OnPickupParticle` "/Game/StarterContent/Particles/P_Explosion.P_Explosion")
  (`GameplayStatics.PlaySoundAtLocation` "/Game/StarterContent/Audio/Fire_Sparks01_Cue.Fire_Sparks01_Cue" (`self.K2_GetActorLocation`) (struct) 1.0 1.0 0.0 null null null)
  (`parent.ReceiveBeginPlay`))

(event `self.OnPickupFunction`
  (params (Object :type "Object Object Reference"))
  (bind _asball_pawn (cast `/Game/Blueprints/BallPawn` Object))
  (`PrimitiveComponent.AddRadialImpulse` (`/Game/Blueprints/BallPawn.Ball Mesh` _asball_pawn) (`KismetMathLibrary.MakeVector` (.x (`self.K2_GetActorLocation`)) (.y (`self.K2_GetActorLocation`)) (+ (.z (`self.K2_GetActorLocation`)) -50.0)) 500.0 1000.0 "RIF_Constant" true)
  (`parent.OnPickupFunction` Object))

(fn `UserConstructionScript`
  (`parent.UserConstructionScript`))